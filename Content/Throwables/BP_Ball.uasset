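; BP_Ball is a throwable that breaks on the floor and leaves a BP_HearingPoint at the impact.
; The Ball component's hit event ignores the player pawn and reacts only to actors tagged Floor.
; A DoOnce gate spawns the hearing point at the hit location, then destroys the ball.
; BeginPlay sets a short lifespan as a fallback cleanup, and an unconnected manual countdown remains unused.
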(event `self.ReceiveBeginPlay`
  (`self.SetLifeSpan` 4.0))

(event `self.ReceiveTick`
  (params (DeltaSeconds :type "Float (single-precision)")))

(event `self.Ball.OnComponentHit`
  (params (HitComponent :type "PrimitiveComponent Object Reference") (OtherActor :type "Actor Object Reference") (OtherComp :type "PrimitiveComponent Object Reference") (NormalImpulse :type "Vector Structure") (Hit :type "HitResult Structure (by ref)"))
  ;[1 1 1] Hit floor and break
  (if (!= OtherActor (`GameplayStatics.GetPlayerPawn` 0))
    (if (`self.ActorHasTag` OtherActor "Floor")
      (`/Engine/EditorBlueprintResources/StandardMacros.DoOnce` false
        (:`Completed`
          (`|SpawnActorFromClass` "/Game/Audio/BP_HearingPoint.BP_HearingPoint_C" (`KismetMathLibrary.Conv_VectorToTransform` Hit_Location) "AdjustIfPossibleButAlwaysSpawn" "MultiplyWithRoot" null null)
          (`self.K2_DestroyActor`))))))

(fn `UserConstructionScript`)