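; BP_BasicEnemy is a basic enemy that turns to face the player while it performs a punch attack.
; It caches the player's BP_ThirdPersonCharacter on BeginPlay.
; The Attacking event prints a debug string, plays the punch montage and starts a fast looping timer that snaps the actor's rotation toward the player.
; Montage completion or interruption clears that timer, as does the StopRotationToPlayer event.
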(event `self.ReceiveBeginPlay`
  (bind _asbp_third_person_character (cast `/Game/ThirdPerson/Blueprints/BP_ThirdPersonCharacter` (`GameplayStatics.GetPlayerCharacter` 0)))
  (set `self.As BP_ThirdPerson` _asbp_third_person_character))

(event `Stop Rotation To Player`
  (`KismetSystemLibrary.K2_ClearAndInvalidateTimerHandle` (`self.RotateTimer`) :!label _label))

(event `Attacking`
  (`KismetSystemLibrary.PrintString` "Enemy Attacking")
  (bind _returnvalue (`KismetSystemLibrary.K2_SetTimerDelegate` (delegate `Rotate to Player`) 0.02 true))
  (set `self.RotateTimer` _returnvalue)
  ;[1 1 1] Animation montage here
  (`|PlayMontage` (`self.Mesh`) "/Game/Enemies/BasicEnemy/Animation/Punching_Montage.Punching_Montage"
    (:`OnCompleted`
      (goto _label))
    (:`OnInterrupted`
      (goto _label))))

(event `Rotate to Player`
  (`self.K2_SetActorRotation` (`KismetMathLibrary.FindLookAtRotation` (`self.K2_GetActorLocation`) (`self.K2_GetActorLocation` (`self.As BP_ThirdPerson`)))))

(fn `UserConstructionScript`)