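; Checkpoint actor that records itself as the LastCheckpoint on BP_ThirdPersonGameMode.
; An instance flagged StartingRoom registers on BeginPlay as the default and ignores player overlaps.
; Other instances register once when the player character overlaps the Trigger, then print a message, play a shutter sound and switch the Cube to a green laser material.
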(event `self.ReceiveBeginPlay`
  ;[1 1 1] Sets starting room as default
  (if (`self.StartingRoom?`)
    (bind _asbp_third_person_game_mode (cast `/Game/ThirdPerson/Blueprints/BP_ThirdPersonGameMode` (`GameplayStatics.GetGameMode`)))
    (set `/Game/ThirdPerson/Blueprints/BP_ThirdPersonGameMode.LastCheckpoint` self _asbp_third_person_game_mode)))

(event `self.Trigger.OnComponentBeginOverlap`
  (params (OverlappedComponent :type "PrimitiveComponent Object Reference") (OtherActor :type "Actor Object Reference") (OtherComp :type "PrimitiveComponent Object Reference") (OtherBodyIndex :type Integer) (bFromSweep :type Boolean) (SweepResult :type "HitResult Structure (by ref)"))
  (if (== OtherActor (`GameplayStatics.GetPlayerCharacter` 0))
    (if (not (`self.StartingRoom?`))
      (`/Engine/EditorBlueprintResources/StandardMacros.DoOnce` false
        (:`Completed`
          (bind _asbp_third_person_game_mode (cast `/Game/ThirdPerson/Blueprints/BP_ThirdPersonGameMode` (`GameplayStatics.GetGameMode`)))
          (set `/Game/ThirdPerson/Blueprints/BP_ThirdPersonGameMode.LastCheckpoint` self _asbp_third_person_game_mode)
          (`KismetSystemLibrary.PrintString` "Checkpoint Reached")
          (`GameplayStatics.PlaySound2D` "/Engine/VREditor/Sounds/UI/Camera_Shutter.Camera_Shutter" 1.0 1.0 0.0 null null)
          (`PrimitiveComponent.SetMaterial` (`self.Cube`) 0 "/Game/Checkpoint/LaserGreen.LaserGreen"))))))

(fn `UserConstructionScript`)