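; BP_Lever is a lever that toggles between two positions each time its PullLever event fires.
; Each pull plays a sound at the actor's location, then a FlipFlop alternately plays or reverses the PullUpAndDown timeline and swaps the Handle's material.
; The timeline's alpha interpolates the Lever component's relative rotation to swing it between the two angles.
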(event `Pull Lever`
  (`GameplayStatics.PlaySoundAtLocation` "/Game/Audio/Sounds/Lever_Sound.Lever_Sound" (`self.K2_GetActorLocation`) (struct) 1.0 1.0 0.0 null null null null)
  (`/Engine/EditorBlueprintResources/StandardMacros.FlipFlop`
    (:`A`
      (`PrimitiveComponent.SetMaterial` (`self.Handle`) 0 "/Engine/MapTemplates/Materials/BasicAsset01.BasicAsset01")
      (bind (_direction _alpha) (`Timeline|Pull Up and Down` :!label _label)
        (:`Update`
          (`SceneComponent.K2_SetRelativeRotation` (`self.Lever`) (`KismetMathLibrary.RLerp` (struct :`Pitch` -30.0) (struct :`Pitch` -130.0) _alpha) false false))))
    (:`B`
      (`PrimitiveComponent.SetMaterial` (`self.Handle`) 0 "/Engine/MapTemplates/Materials/BasicAsset03.BasicAsset03")
      (goto _label :!via `Reverse`))))

(fn `UserConstructionScript`)