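; BP_SingleDoor is a sliding metal door that opens or closes when triggered through an interface event.
; Each OpenDoor call plays a sound and flips a FlipFlop that plays or reverses a timeline, lerping the door mesh's relative location.
; If SelfCloseEnabled is set, the player's first overlap with the AutoClose component toggles that same FlipFlop once, skipping the sound.
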(event `/Game/Levers/BPI_DoorInteract.BPI_OpenDoor`
  (`self.Open Door`))

(event `self.ReceiveBeginPlay`)

(event `Open Door`
  (`GameplayStatics.PlaySoundAtLocation` "/Game/Audio/Sounds/Metal_Door_Move.Metal_Door_Move" (`self.K2_GetActorLocation`) (struct) 1.0 1.0 0.0 null null null null)
  (`/Engine/EditorBlueprintResources/StandardMacros.FlipFlop` :!label _label
    (:`A`
      (bind (_direction _door_open) (`Timeline|OpenDoorAnim` :!label _label_2)
        (:`Update`
          (`SceneComponent.K2_SetRelativeLocation` (`self.SM_DoorLeft`) (`KismetMathLibrary.VLerp` (0.0 210.0 0.0) (0.0 660.0 0.0) _door_open) false false))))
    (:`B`
      (goto _label_2 :!via `Reverse`))))

(event `self.Auto Close.OnComponentBeginOverlap`
  (params (OverlappedComponent :type "PrimitiveComponent Object Reference") (OtherActor :type "Actor Object Reference") (OtherComp :type "PrimitiveComponent Object Reference") (OtherBodyIndex :type Integer) (bFromSweep :type Boolean) (SweepResult :type "HitResult Structure (by ref)"))
  (if (`self.SelfCloseEnabled?`)
    (if (== OtherActor (`GameplayStatics.GetPlayerCharacter` 0))
      (`/Engine/EditorBlueprintResources/StandardMacros.DoOnce` false
        (:`Completed`
          (goto _label))))))

(fn `UserConstructionScript`)