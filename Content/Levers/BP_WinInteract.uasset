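; BP_WinInteract is a win trigger actor that ends play with a victory screen when the player enters its box.
; It caches the third-person character on BeginPlay.
; On box overlap by player 0, it sets that character's IsGameOver to false and starts a held camera fade.
; It then creates and shows the PlayerWin_WBP widget, switching to UI-only input with a visible cursor.
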(event `self.ReceiveBeginPlay`
  (bind _asbp_third_person_character (cast `/Game/ThirdPerson/Blueprints/BP_ThirdPersonCharacter` (`GameplayStatics.GetPlayerCharacter` 0)))
  (set `self.As BP Third Person Character` _asbp_third_person_character))

(event `self.Box.OnComponentBeginOverlap`
  (params (OverlappedComponent :type "PrimitiveComponent Object Reference") (OtherActor :type "Actor Object Reference") (OtherComp :type "PrimitiveComponent Object Reference") (OtherBodyIndex :type Integer) (bFromSweep :type Boolean) (SweepResult :type "HitResult Structure (by ref)"))
  (bind _returnvalue (`GameplayStatics.GetPlayerController` 0))
  (if (== OtherActor (`GameplayStatics.GetPlayerCharacter` 0))
    (set `/Game/ThirdPerson/Blueprints/BP_ThirdPersonCharacter.IsGameOver` false (`self.As BP Third Person Character`))
    (`PlayerCameraManager.StartCameraFade` :`self` (`GameplayStatics.GetPlayerCameraManager` 0) :`ToAlpha` 1.0 :`Duration` 2.0 :`bHoldWhenFinished` true)
    (bind _returnvalue_2 (`|GenericCreateObject` (`GameplayStatics.GetPlayerController` 0) "/Game/UI/PlayerWin_WBP.PlayerWin_WBP_C"))
    (bind _output_get (set `self.PlayerWinRef` _returnvalue_2))
    (`UserWidget.AddToViewport` _output_get 0)
    (`WidgetBlueprintLibrary.SetInputMode_UIOnlyEx` _returnvalue (`self.PlayerWinRef`) "DoNotLock" true)
    (set `PlayerController.bShowMouseCursor` true _returnvalue)))

(fn `UserConstructionScript`)