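; BP_DoubleDoor is a sliding double door that opens or closes when triggered through an interface event.
; Each trigger plays a metal door sound, and a FlipFlop alternately plays or reverses a timeline.
; The timeline lerps the left and right meshes' relative locations apart in opposite directions along Y.
; An auto-close overlap event exists but is empty, and its player-check and delay logic is disconnected.
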(event `/Game/Levers/BPI_DoorInteract.BPI_OpenDoubleDoor`
  (`self.Open Double Door`))

(event `self.ReceiveBeginPlay`)

(event `Open Double Door`
  (`GameplayStatics.PlaySoundAtLocation` "/Game/Audio/Sounds/Metal_Door_Move.Metal_Door_Move" (`self.K2_GetActorLocation`) (struct) 1.0 1.0 0.0 null null null null)
  (`/Engine/EditorBlueprintResources/StandardMacros.FlipFlop`
    (:`A`
      (bind (_direction _door_open) (`Timeline|OpenDoorAnim` :!label _label)
        (:`Update`
          (`SceneComponent.K2_SetRelativeLocation` (`self.SM_DoorRight`) (`KismetMathLibrary.VLerp` (0.0 0.0 0.0) (0.0 180.0 0.0) _door_open) false false)
          (`SceneComponent.K2_SetRelativeLocation` (`self.SM_DoorLeft`) (`KismetMathLibrary.VLerp` (0.0 0.0 0.0) (0.0 -180.0 0.0) _door_open) false false))))
    (:`B`
      (goto _label :!via `Reverse`))))

(event `self.Auto Close.OnComponentBeginOverlap`
  (params (OverlappedComponent :type "PrimitiveComponent Object Reference") (OtherActor :type "Actor Object Reference") (OtherComp :type "PrimitiveComponent Object Reference") (OtherBodyIndex :type Integer) (bFromSweep :type Boolean) (SweepResult :type "HitResult Structure (by ref)")))

(fn `UserConstructionScript`)